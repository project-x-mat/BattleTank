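; Player-controllable tank pawn Blueprint that routes input to aiming, movement and track components.
; On BeginPlay it hands the barrel and turret to TankAIming and both tracks to TankMovement.
; Aim axes rotate the spring arm, yaw in world space and pitch in local space.
; Driving works through movement intents or direct per-track throttle, and Fire calls TankAIming.
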(event EventBeginPlay
  (Class|TankAImingComponent|Initialize (Variables|Default|GetTankAIming) (Variables|Default|GetBarrel) (Variables|Default|GetTankTurret))
  (Class|TankMovementComponent|Initialize (Variables|Default|GetTankMovement) (Variables|Default|GetLeftTrack) (Variables|Default|GetRightTrack)))

(event Input|ActionEvents|InputActionFire
  (params (Key :type Key%20Structure))
  ;[1 1 1] Input SetupSetup
  (:Pressed
    (Class|TankAImingComponent|Fire (Variables|Default|GetTankAIming))))

(event Input|AxisEvents|InputAxisAimAzimuth
  (params (AxisValue :type Float%20%28single-precision%29))
  ;[1 1 1] Input SetupSetup
  (Transformation|AddWorldRotation (Variables|Default|GetSpringArm) (Math|Rotator|MakeRotator 0.0 0.0 AxisValue) false false))

(event Input|AxisEvents|InputAxisAimElavation
  (params (AxisValue :type Float%20%28single-precision%29))
  ;[1 1 1] Input SetupSetup
  (Transformation|AddLocalRotation (Variables|Default|GetSpringArm) (Math|Rotator|MakeRotator 0.0 AxisValue 0.0) false false))

(event Input|AxisEvents|InputAxisMoveForward
  (params (AxisValue :type Float%20%28single-precision%29))
  ;[1 1 1] Input binding
  (Class|TankMovementComponent|IntendMoveForward (Variables|Default|GetTankMovement) AxisValue))

(event Input|AxisEvents|InputAxisTurnRight
  (params (AxisValue :type Float%20%28single-precision%29))
  ;[1 1 1] Input binding
  (Class|TankMovementComponent|IntendTurnRight (Variables|Default|GetTankMovement) AxisValue))

(event Input|AxisEvents|InputAxisLefttrackThrottle
  (params (AxisValue :type Float%20%28single-precision%29))
  ;[1 1 1] Input binding
  (Class|TankTrack|SetThrottle (Variables|Default|GetLeftTrack) AxisValue))

(event Input|AxisEvents|InputAxisRightTackThrottle
  (params (AxisValue :type Float%20%28single-precision%29))
  ;[1 1 1] Input binding
  (Class|TankTrack|SetThrottle (Variables|Default|GetRightTrack) AxisValue))

(fn ConstructionScript)